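; BP_Helix is an actor whose static mesh spins while the player character reports an active helix-related interaction.
; Each Tick it reads the HasInteractH and HasInputH flags from BP_ThirdPersonCharacterVirgile.
; When both are true, it adds a fixed roll increment to the mesh's relative rotation, so spin speed depends on frame rate.
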(event `self.ReceiveTick`
  (params (DeltaSeconds :type "Float (single-precision)"))
  (bind _asbp_third_person_character_virgile (cast `/Game/DepthScape/Virgile/Blueprints/BP_ThirdPersonCharacterVirgile` (`GameplayStatics.GetPlayerCharacter` 0) :!pure true))
  (bind (_relativerotation_roll _relativerotation_pitch _relativerotation_yaw) (`KismetMathLibrary.BreakRotator` (`SceneComponent.RelativeRotation` (`self.StaticMesh`))))
  (if (and (`/Game/DepthScape/Virgile/Blueprints/BP_ThirdPersonCharacterVirgile.hasInteractH` _asbp_third_person_character_virgile) (`/Game/DepthScape/Virgile/Blueprints/BP_ThirdPersonCharacterVirgile.hasInputH` _asbp_third_person_character_virgile))
    (`SceneComponent.K2_SetRelativeRotation` (`self.StaticMesh`) (`KismetMathLibrary.MakeRotator` (+ _relativerotation_roll 0.2) _relativerotation_pitch _relativerotation_yaw) false false)))

(fn `UserConstructionScript`)