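; Blueprint function library that reports whether the local player is using a gamepad or a keyboard.
; DetectGamepad and DetectKeyboard each cast player controller 0 to BP_PyritePlayerController and return its IsUsingGamepad or IsUsingKeyboard flag.
; The library only reads these flags and does no input detection of its own.
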(fn `DetectGamepad`
  (returns (isUsingGamepad :type Boolean))
  (bind _asbp_pyrite_player_controller (cast `/Game/DepthScape/Patrick/BP_PyritePlayerController` (`GameplayStatics.GetPlayerController` null)))
  (if (`/Game/DepthScape/Patrick/BP_PyritePlayerController.isUsingGamepad` _asbp_pyrite_player_controller)
    (return true)
    (else
      (return false))))

(fn `DetectKeyboard`
  (returns (isUsingKeyboard :type Boolean))
  (bind _asbp_pyrite_player_controller (cast `/Game/DepthScape/Patrick/BP_PyritePlayerController` (`GameplayStatics.GetPlayerController` null)))
  (if (`/Game/DepthScape/Patrick/BP_PyritePlayerController.isUsingKeyboard` _asbp_pyrite_player_controller)
    (return true)
    (else
      (return false))))