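; Trigger volume that starts a screen fade on the player's HUD; despite its name, it contains no level-opening call.
; On Box begin overlap, it compares the overlapping actor to the BP_ProtoPatrick player's capsule component.
; A match switches the HUD's outline widget switcher and calls FadeIn on WBPFade.
; End overlap is empty, and a matching FadeOut branch is left unconnected.
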(event `self.Box.OnComponentBeginOverlap`
  (params (OverlappedComponent :type "PrimitiveComponent Object Reference") (OtherActor :type "Actor Object Reference") (OtherComp :type "PrimitiveComponent Object Reference") (OtherBodyIndex :type Integer) (bFromSweep :type Boolean) (SweepResult :type "HitResult Structure (by ref)"))
  (bind _asbp_proto_patrick (cast `/Game/DepthScape/Patrick/Blueprints/Character/BP_ProtoPatrick` (`GameplayStatics.GetPlayerCharacter` 0) :!pure true))
  (bind _characterhudwidget (`/Game/DepthScape/Patrick/Blueprints/Character/BP_ProtoPatrick.CharacterHUDWidget` _asbp_proto_patrick))
  (if (== OtherActor (`Character.CapsuleComponent` _asbp_proto_patrick))
    (`WidgetSwitcher.SetActiveWidgetIndex` (`/Game/DepthScape/Patrick/Widgets/WBP_CharacterHUD.WidgetSwitcher_Outline` _characterhudwidget) 3)
    (`/Game/DepthScape/Virgile/UI/Widgets/WBP_Fade.Fade_In` (`/Game/DepthScape/Patrick/Widgets/WBP_CharacterHUD.WBP_Fade` _characterhudwidget))))

(event `self.Box.OnComponentEndOverlap`
  (params (OverlappedComponent :type "PrimitiveComponent Object Reference") (OtherActor :type "Actor Object Reference") (OtherComp :type "PrimitiveComponent Object Reference") (OtherBodyIndex :type Integer)))

(fn `UserConstructionScript`)