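; BP_Pheromone is a thrown projectile whose effect on impact depends on its throw mutation: Bloom, Flash, Sting Trap or Stunning Slingshot.
; BeginPlay launches it and picks the mesh material from the player's equipped throw type, while hit handling switches on its own ThrowMutations variable.
; Bloom spawns an animated BP_Bush on upward-facing surfaces.
; The others destroy it on hit, with Flash and Sting triggering BP_Watcher reactions and Stunning only printing.
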(event `self.ReceiveBeginPlay`
  (set `MovementComponent.Velocity` (`self.Velocity`) (`self.ProjectileMovement`))
  (`SceneComponent.SetWorldScale3D` (`self.StaticMesh`) (0.15 0.15 0.15))
  (switch `/Game/DepthScape/Virgile/Blueprints/EThrowMutations` (`/Game/DepthScape/Patrick/Blueprints/Character/BP_PyriteCharacter.EquipedThrowType` (cast `/Game/DepthScape/Patrick/Blueprints/Character/BP_PyriteCharacter` (`GameplayStatics.GetPlayerCharacter` 0) :!pure true))
    (:`NewEnumerator0`
      (`PrimitiveComponent.SetMaterial` (`self.StaticMesh`) 0 "/Game/DepthScape/Patrick/Assets/Materials/MI_BushV2.MI_BushV2")
      (`KismetSystemLibrary.PrintString` (`|GetEnumeratorNameAsString` (`self.ThrowMutations`))))
    (:`NewEnumerator1`
      (`PrimitiveComponent.SetMaterial` (`self.StaticMesh`) 0 "/Game/DepthScape/Virgile/VFX/M_SmokeBall.M_SmokeBall")
      (`KismetSystemLibrary.PrintString` (`|GetEnumeratorNameAsString` (`self.ThrowMutations`))))
    (:`NewEnumerator2`
      (`PrimitiveComponent.SetMaterial` (`self.StaticMesh`) 0 null)
      (`KismetSystemLibrary.PrintString` (`|GetEnumeratorNameAsString` (`self.ThrowMutations`))))
    (:`NewEnumerator3`
      (`PrimitiveComponent.SetMaterial` (`self.StaticMesh`) 0 "/Game/StarterContent/Materials/M_Rock_Basalt.M_Rock_Basalt")
      (`KismetSystemLibrary.PrintString` (`|GetEnumeratorNameAsString` (`self.ThrowMutations`))))))

(event `self.StaticMesh.OnComponentHit`
  (params (HitComponent :type "PrimitiveComponent Object Reference") (OtherActor :type "Actor Object Reference") (OtherComp :type "PrimitiveComponent Object Reference") (NormalImpulse :type "Vector Structure") (Hit :type "HitResult Structure (by ref)"))
  (switch `/Game/DepthScape/Virgile/Blueprints/EThrowMutations` (`self.ThrowMutations`)
    (:`NewEnumerator0`
      (if (== Hit_Normal (0.0 0.0 1.0) :`ErrorTolerance` 0.2)
        (`self.SpawnBush`)))
    (:`NewEnumerator1`
      (bind _asbp_watcher (cast `/Game/DepthScape/Patrick/Blueprints/Enemy/Watcher/BP_Watcher` OtherActor)
        (:`then`
          ;[1 0 0 1 30] Flash Event
          (`/Game/DepthScape/Patrick/Blueprints/Enemy/Watcher/BPAI_Watcher.Flash Event` (`/Game/DepthScape/Patrick/Blueprints/Enemy/Watcher/BP_Watcher.GetAIControllerClass` _asbp_watcher))
          (`/Game/DepthScape/Patrick/Blueprints/Enemy/Watcher/BP_Watcher.PlayFlashVFX` _asbp_watcher)
          (`self.K2_DestroyActor`))
        (:`CastFailed`
          (`self.K2_DestroyActor`))))
    (:`NewEnumerator2`
      (bind _asbp_watcher_2 (cast `/Game/DepthScape/Patrick/Blueprints/Enemy/Watcher/BP_Watcher` OtherActor)
        (:`then`
          ;[1 0 0 1 30] Sting Trap Event
          (`/Game/DepthScape/Patrick/Blueprints/Enemy/Watcher/BP_Watcher.Sting Trap Event` _asbp_watcher_2)
          (`/Game/DepthScape/Patrick/Blueprints/Enemy/Watcher/BP_Watcher.PlayStingVFX` _asbp_watcher_2)
          (`self.K2_DestroyActor`))
        (:`CastFailed`
          (`self.K2_DestroyActor`))))
    (:`NewEnumerator3`
      (cast `/Game/DepthScape/Patrick/Blueprints/Enemy/Watcher/BP_Watcher` OtherActor
        (:`then`
          ;[1 0 0 1 30] Stunning Event
          (`KismetSystemLibrary.PrintString` "Stunning")
          (`self.K2_DestroyActor`))
        (:`CastFailed`
          (`self.K2_DestroyActor`))))))

(event `SpawnBush`
  (bind (_returnvalue_x _returnvalue_y _returnvalue_z) (`KismetMathLibrary.BreakVector` (`SceneComponent.K2_GetComponentLocation` (`self.Scene`))))
  (bind _returnvalue (`|SpawnActorFromClass` "/Game/DepthScape/Patrick/Blueprints/Environments/BP_Bush.BP_Bush_C" (`KismetMathLibrary.MakeTransform` (`KismetMathLibrary.MakeVector` _returnvalue_x _returnvalue_y (- _returnvalue_z 40.0)) (struct) (0.0 0.0 0.0)) "AdjustIfPossibleButAlwaysSpawn" "MultiplyWithRoot" null null))
  (bind _output_get (set `self.Bush` _returnvalue))
  (`/Game/DepthScape/Patrick/Blueprints/Environments/BP_Bush.SpawnAnimation` _output_get)
  (`self.K2_DestroyActor`))

(fn `UserConstructionScript`)