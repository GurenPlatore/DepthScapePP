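; BP_Elevator is an elevator that moves its static mesh between a start and an end location when the player interacts.
; BeginPlay stores the mesh's relative location as StartLoc, and Tick polls HasInteractE on BP_ThirdPersonCharacterVirgile with no proximity check in the graph.
; While that flag is true, Tick plays Timeline, whose every update sets the lerped location and also plays Timeline_0, which writes the same lerp using its own track.
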(event `self.ReceiveBeginPlay`
  (set `self.StartLoc` (`SceneComponent.RelativeLocation` (`self.StaticMesh`))))

(event `self.ReceiveTick`
  (params (DeltaSeconds :type "Float (single-precision)"))
  (if (`/Game/DepthScape/Virgile/Blueprints/BP_ThirdPersonCharacterVirgile.hasInteractE` (cast `/Game/DepthScape/Virgile/Blueprints/BP_ThirdPersonCharacterVirgile` (`GameplayStatics.GetPlayerCharacter` 0) :!pure true))
    (bind (_direction _newtrack_0) (`Timeline|Timeline`)
      (:`Update`
        (`SceneComponent.K2_SetRelativeLocation` (`self.StaticMesh`) (`KismetMathLibrary.VLerp` (`self.StartLoc`) (`self.EndLoc`) _newtrack_0) false false)
        (bind (_direction_2 _newtrack_0_2) (`Timeline|Timeline_0`)
          (:`Update`
            (`SceneComponent.K2_SetRelativeLocation` (`self.StaticMesh`) (`KismetMathLibrary.VLerp` (`self.StartLoc`) (`self.EndLoc`) _newtrack_0_2) false false)))))))

(fn `UserConstructionScript`)