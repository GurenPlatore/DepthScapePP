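; BP_BulbacideTrigger is a one-shot hold-to-interact trigger that makes a referenced Bulbacide spawn gas during a camera cutaway.
; Box overlap toggles the interaction widget for the Pyrite character.
; External StartTickInteraction calls raise progress and enable Tick, which drains it, updates the bar and sleeps at zero.
; Near full, it disables itself, blends to its camera and back, and freezes player movement on a separate fixed delay.
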(event `self.ReceiveTick`
  (params (DeltaSeconds :type "Float (single-precision)"))
  (if (`self.isComplete`)
    _
    (elif (== (`self.ProgressValue`) 0.0)
      (`self.SetActorTickEnabled` false)
      (`self.HideProgressBar`)
      (elif (`KismetMathLibrary.NearlyEqual_FloatFloat` (`self.ProgressValue`) 1.0 0.01)
        (`CharacterMovementComponent.DisableMovement` (`self.GetCharacterMovement`))
        (`self.SetActorTickEnabled` false)
        (`PrimitiveComponent.SetCollisionEnabled` (`self.Box`) "NoCollision")
        (`SceneComponent.SetVisibility` (`self.WidgetInteraction`) false false)
        (`self.DisablePlayerMovement`)
        (`PlayerController.SetViewTargetWithBlend` (`GameplayStatics.GetPlayerController` 0) (`self.Camera`) 2.0 "VTBlend_Cubic" 2.0 false)
        (`KismetSystemLibrary.Delay` 2.0)
        (`/Game/DepthScape/Virgile/Blueprints/BP_Bulbacide.SpawnGas` (`self.BulbacideREF`))
        (`KismetSystemLibrary.Delay` (`self.Duration`))
        (`PlayerController.SetViewTargetWithBlend` (`GameplayStatics.GetPlayerController` 0) (`GameplayStatics.GetPlayerCharacter` 0) 5.0 "VTBlend_Cubic" 5.0 false)
        (set `self.isComplete` true)
        (`KismetSystemLibrary.Delay` 3.0)
        (`CharacterMovementComponent.SetMovementMode` (`self.GetCharacterMovement`) "MOVE_Walking" 0)
        (else
          (`self.HoldInteraction` DeltaSeconds)
          (`self.DisplayProgressBar`))))))

(event `self.ReceiveBeginPlay`
  (`self.HideProgressBar`))

(event `self.Box.OnComponentBeginOverlap`
  (params (OverlappedComponent :type "PrimitiveComponent Object Reference") (OtherActor :type "Actor Object Reference") (OtherComp :type "PrimitiveComponent Object Reference") (OtherBodyIndex :type Integer) (bFromSweep :type Boolean) (SweepResult :type "HitResult Structure (by ref)"))
  (cast `/Game/DepthScape/Patrick/Blueprints/Character/BP_PyriteCharacter` OtherActor)
  (`SceneComponent.SetVisibility` (`self.WidgetInteraction`) true false))

(event `self.Box.OnComponentEndOverlap`
  (params (OverlappedComponent :type "PrimitiveComponent Object Reference") (OtherActor :type "Actor Object Reference") (OtherComp :type "PrimitiveComponent Object Reference") (OtherBodyIndex :type Integer))
  (cast `/Game/DepthScape/Patrick/Blueprints/Character/BP_PyriteCharacter` OtherActor)
  (`SceneComponent.SetVisibility` (`self.WidgetInteraction`) false false))

(fn `DisablePlayerMovement`
  (`CharacterMovementComponent.DisableMovement` (`Character.CharacterMovement` (cast `/Game/DepthScape/Patrick/Blueprints/Character/BP_PyriteCharacter` (`GameplayStatics.GetPlayerCharacter` 0) :!pure true))))

(fn `DisplayProgressBar`
  (`SceneComponent.SetVisibility` (`self.WidgetInteraction`) true false))

(fn `GetCharacterMovement`
  (returns (CharacterMovement :type "CharacterMovementComponent Object Reference"))
  (return (`Character.CharacterMovement` (cast `/Game/DepthScape/Patrick/Blueprints/Character/BP_PyriteCharacter` (`GameplayStatics.GetPlayerCharacter` 0) :!pure true))))

(fn `HideProgressBar`
  (`SceneComponent.SetVisibility` (`self.WidgetInteraction`) false false))

(fn `HoldInteraction`
  (params (Delta :type "Float (double-precision)"))
  (set `self.ProgressValue` (`KismetMathLibrary.FClamp` (- (`self.ProgressValue`) (/ Delta 3.0))))
  (bind _aswbp_interact (cast `/Game/DepthScape/Virgile/UI/Widgets/WBP_Interact` (`WidgetComponent.GetWidget` (`self.WidgetInteraction`))))
  (`/Game/DepthScape/Virgile/UI/Widgets/Overlay/WBP_CircularProgressBar.SetPercent` (`/Game/DepthScape/Virgile/UI/Widgets/WBP_Interact.WBP_ProgressBarMutation` _aswbp_interact) (`self.ProgressValue`)))

(fn `SetPlayerMovementMode`
  (params (NewMovementMode :type "EMovementMode Enum" :default "MOVE_None"))
  (`CharacterMovementComponent.SetMovementMode` (`Character.CharacterMovement` (cast `/Game/DepthScape/Patrick/Blueprints/Character/BP_PyriteCharacter` (`GameplayStatics.GetPlayerCharacter` 0) :!pure true)) NewMovementMode 0))

(fn `StartTickInteraction`
  (`self.SetActorTickEnabled` true)
  (set `self.ProgressValue` (`KismetMathLibrary.FClamp` (+ (`self.ProgressValue`) 0.01))))

(fn `UserConstructionScript`
  (`parent.UserConstructionScript`))