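; BP_EndTrigger is a box trigger that plays the ending when BP_PyriteCharacter enters it.
; It creates WBP_EndingWidget at BeginPlay, then on overlap disables character movement, clears all widgets, blends the view to its Camera and shows the ending widget two seconds later.
; A five-second cubic blend to the player character is issued first, but the camera blend follows it without any delay.
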(event `self.ReceiveBeginPlay`
  (bind _returnvalue (`|CreateWidget` "/Game/DepthScape/Virgile/UI/Widgets/WBP_EndingWidget.WBP_EndingWidget_C"))
  (set `self.EndingWidget` _returnvalue))

(event `self.Box.OnComponentBeginOverlap`
  (params (OverlappedComponent :type "PrimitiveComponent Object Reference") (OtherActor :type "Actor Object Reference") (OtherComp :type "PrimitiveComponent Object Reference") (OtherBodyIndex :type Integer) (bFromSweep :type Boolean) (SweepResult :type "HitResult Structure (by ref)"))
  (bind _asbp_pyrite_character (cast `/Game/DepthScape/Patrick/Blueprints/Character/BP_PyriteCharacter` OtherActor))
  (`PlayerController.SetViewTargetWithBlend` (`GameplayStatics.GetPlayerController` 0) (`GameplayStatics.GetPlayerCharacter` 0) 5.0 "VTBlend_Cubic" 5.0 false)
  (`CharacterMovementComponent.DisableMovement` (`Character.CharacterMovement` _asbp_pyrite_character))
  (`WidgetLayoutLibrary.RemoveAllWidgets`)
  (`PlayerController.SetViewTargetWithBlend` (`GameplayStatics.GetPlayerController` 0) (`self.Camera`) 2.0 "VTBlend_Linear" 0.0 false)
  (`KismetSystemLibrary.Delay` 2.0)
  (`UserWidget.AddToViewport` (`self.EndingWidget`) 0))

(fn `UserConstructionScript`)