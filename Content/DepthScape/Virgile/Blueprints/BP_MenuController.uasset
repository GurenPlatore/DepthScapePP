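; BP_MenuController is a menu controller that tracks whether the most recent key press comes from a keyboard or a gamepad.
; An AnyKey press event classifies the key and sets the mutually exclusive IsUsingKeyboard and IsUsingGamepad flags, leaving them unchanged for other key types.
; Each press first prints both flags as debug text, so the output shows the state before the update.
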(event `Key|AnyKey`
  (params (Key :type "Key Structure"))
  (:`Pressed`
    (`KismetSystemLibrary.PrintString` (`KismetStringLibrary.Concat_StrStr` (`KismetStringLibrary.Conv_BoolToString` (`self.isUsingGamepad`)) " : " (`KismetStringLibrary.Conv_BoolToString` (`self.isUsingKeyboard`))))
    (if (`KismetInputLibrary.Key_IsKeyboardKey` Key)
      (set `self.isUsingKeyboard` true)
      (set `self.isUsingGamepad` false)
      (elif (`KismetInputLibrary.Key_IsGamepadKey` Key)
        (set `self.isUsingGamepad` true)
        (set `self.isUsingKeyboard` false)))))

(fn `UserConstructionScript`)