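; Vent actor that carries BP_PyriteCharacter between two ends of a spline tunnel, in either direction.
; Overlap boxes at each end store the character, set a flag and show a widget.
; StartVentBox and EndVentBox disable input, hide the character's root component and switch view to the vent camera.
; Separate timelines move that camera along the spline forward or backward, then teleport the character to the opposite end and restore view and input.
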(event `SwitchCamera`
  (params (NewViewTarget :type "Actor Object Reference"))
  (`PlayerController.SetViewTargetWithBlend` (`GameplayStatics.GetPlayerController` 0) NewViewTarget 0.0 "VTBlend_Linear" 0.0 false))

(event `self.StartBox.OnComponentBeginOverlap`
  (params (OverlappedComponent :type "PrimitiveComponent Object Reference") (OtherActor :type "Actor Object Reference") (OtherComp :type "PrimitiveComponent Object Reference") (OtherBodyIndex :type Integer) (bFromSweep :type Boolean) (SweepResult :type "HitResult Structure (by ref)"))
  (bind _asbp_pyrite_character (cast `/Game/DepthScape/Patrick/Blueprints/Character/BP_PyriteCharacter` OtherActor))
  (set `self.CharacterREF` _asbp_pyrite_character)
  (set `self.isStarted` true)
  (`SceneComponent.SetVisibility` (`self.StartWidget`) true false))

(event `self.StartBox.OnComponentEndOverlap`
  (params (OverlappedComponent :type "PrimitiveComponent Object Reference") (OtherActor :type "Actor Object Reference") (OtherComp :type "PrimitiveComponent Object Reference") (OtherBodyIndex :type Integer))
  (cast `/Game/DepthScape/Patrick/Blueprints/Character/BP_PyriteCharacter` OtherActor)
  (set `self.isStarted` false)
  (`SceneComponent.SetVisibility` (`self.StartWidget`) false false))

(event `self.EndBox.OnComponentBeginOverlap`
  (params (OverlappedComponent :type "PrimitiveComponent Object Reference") (OtherActor :type "Actor Object Reference") (OtherComp :type "PrimitiveComponent Object Reference") (OtherBodyIndex :type Integer) (bFromSweep :type Boolean) (SweepResult :type "HitResult Structure (by ref)"))
  (bind _asbp_pyrite_character (cast `/Game/DepthScape/Patrick/Blueprints/Character/BP_PyriteCharacter` OtherActor))
  (set `self.CharacterREF` _asbp_pyrite_character)
  (set `self.isEnded` true)
  (`SceneComponent.SetVisibility` (`self.EndWidget`) true false))

(event `self.EndBox.OnComponentEndOverlap`
  (params (OverlappedComponent :type "PrimitiveComponent Object Reference") (OtherActor :type "Actor Object Reference") (OtherComp :type "PrimitiveComponent Object Reference") (OtherBodyIndex :type Integer))
  (cast `/Game/DepthScape/Patrick/Blueprints/Character/BP_PyriteCharacter` OtherActor)
  (set `self.isEnded` false)
  (`SceneComponent.SetVisibility` (`self.EndWidget`) false false))

(event `StartVentBox`
  (bind _spline (`self.Spline`))
  (`SceneComponent.SetVisibility` (`Actor.RootComponent` (`self.CharacterREF`)) false false)
  (`self.DisableInput` (`self.CharacterREF`) (`GameplayStatics.GetPlayerController` 0))
  (`self.SwitchCamera` self)
  (`TimelineComponent.SetPlayRate` (`self.Timeline`) (/ 0.5 (`self.Speed`)))
  (if (== (`self.isActive`) false)
    (bind (_direction _percentage) (`Timeline|Timeline` :!label _label)
      (:`Update`
        (bind _returnvalue (* _percentage (`SplineComponent.GetSplineLength` _spline)))
        (`SceneComponent.K2_SetWorldLocationAndRotation` (`self.Camera`) (`SplineComponent.GetLocationAtDistanceAlongSpline` _spline _returnvalue "World") (`SplineComponent.GetRotationAtDistanceAlongSpline` _spline _returnvalue "Local") false false))
      (:`Finished`
        (`PlayerController.SetViewTargetWithBlend` (`GameplayStatics.GetPlayerController` 0) (`self.CharacterREF`) 0.0 "VTBlend_Linear" 0.0 false)
        (`SceneComponent.K2_SetWorldLocation` (`Character.CapsuleComponent` (`self.CharacterREF`)) (`SceneComponent.K2_GetComponentLocation` (`self.EndLocation`)) false true)
        (set `self.isActive` true)
        (`self.EnableInput` (`self.CharacterREF`) (`GameplayStatics.GetPlayerController` 0))
        (set `self.isStarted` false)))
    (else
      (goto _label :!via `PlayFromStart`))))

(event `EndVentBox`
  (bind _camera (`self.Camera`))
  (bind _spline (`self.Spline`))
  (bind (_relativerotation_roll _relativerotation_pitch _relativerotation_yaw) (`KismetMathLibrary.BreakRotator` (`SceneComponent.RelativeRotation` _camera)))
  (`SceneComponent.SetVisibility` (`Actor.RootComponent` (`self.CharacterREF`)) false false)
  (`self.DisableInput` (`self.CharacterREF`) (`GameplayStatics.GetPlayerController` 0))
  (`SceneComponent.K2_SetWorldRotation` _camera (`KismetMathLibrary.MakeRotator` (+ _relativerotation_roll 545.0) _relativerotation_pitch (+ _relativerotation_yaw 1210.0)) true true)
  (`self.SwitchCamera` self)
  (`TimelineComponent.SetPlayRate` (`self.Timeline`) (/ 0.5 (`self.Speed`)))
  (if (not (`self.isActive`))
    (bind (_direction _percentage) (`Timeline|Timeline_0` :!via `Reverse` :!label _label_2)
      (:`Update`
        (bind _returnvalue (* _percentage (`SplineComponent.GetSplineLength` _spline)))
        (`SceneComponent.K2_SetWorldLocationAndRotation` (`self.Camera`) (`SplineComponent.GetLocationAtDistanceAlongSpline` _spline _returnvalue "World") (`SplineComponent.GetRotationAtDistanceAlongSpline` _spline _returnvalue "Local") false true))
      (:`Finished`
        (`PlayerController.SetViewTargetWithBlend` (`GameplayStatics.GetPlayerController` 0) (`self.CharacterREF`) 0.0 "VTBlend_Linear" 0.0 false)
        (`SceneComponent.K2_SetWorldLocation` (`Character.CapsuleComponent` (`self.CharacterREF`)) (`SceneComponent.K2_GetComponentLocation` (`self.StartLocation`)) false true)
        (set `self.isActive` true)
        (`self.EnableInput` (`self.CharacterREF`) (`GameplayStatics.GetPlayerController` 0))
        (set `self.isEnded` false)))
    (else
      (goto _label_2 :!via `ReverseFromEnd`))))

(fn `UserConstructionScript`)