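; BP_MutationsBath is a world actor that serves as the access point to the mutations menu.
; A box overlap with BP_ProtoPatrick shows or hides the actor's widget component.
; The OpenMutationsMenu event creates WBP_MutationsMenu, adds it to the viewport, and switches the first player controller to UI-only input with a visible cursor.
; Nothing in this graph calls that event or closes the menu.
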(event `OpenMutationsMenu`
  (bind _returnvalue (`GameplayStatics.GetPlayerController` 0))
  (bind _returnvalue_2 (`|CreateWidget` "/Game/DepthScape/Virgile/UI/Widgets/Menu/WBP_MutationsMenu.WBP_MutationsMenu_C"))
  (`UserWidget.AddToViewport` _returnvalue_2 0)
  (`WidgetBlueprintLibrary.SetInputMode_UIOnlyEx` _returnvalue null)
  (set `PlayerController.bShowMouseCursor` true _returnvalue))

(event `self.Box.OnComponentBeginOverlap`
  (params (OverlappedComponent :type "PrimitiveComponent Object Reference") (OtherActor :type "Actor Object Reference") (OtherComp :type "PrimitiveComponent Object Reference") (OtherBodyIndex :type Integer) (bFromSweep :type Boolean) (SweepResult :type "HitResult Structure (by ref)"))
  (cast `/Game/DepthScape/Patrick/Blueprints/Character/BP_ProtoPatrick` OtherActor)
  (`SceneComponent.SetVisibility` (`self.Widget`) true false))

(event `self.Box.OnComponentEndOverlap`
  (params (OverlappedComponent :type "PrimitiveComponent Object Reference") (OtherActor :type "Actor Object Reference") (OtherComp :type "PrimitiveComponent Object Reference") (OtherBodyIndex :type Integer))
  (cast `/Game/DepthScape/Patrick/Blueprints/Character/BP_ProtoPatrick` OtherActor)
  (`SceneComponent.SetVisibility` (`self.Widget`) false false))

(fn `UserConstructionScript`
  (`parent.UserConstructionScript`))