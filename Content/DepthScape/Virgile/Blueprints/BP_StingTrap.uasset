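; BP_StingTrap is a sting trap actor that plays a spawn animation with a particle burst and a scale change.
; BeginPlay binds SpawnAnimation to OnSpawn, which spawns the NS_StingTrapV2 system just above the root's relative location.
; After a short delay, a Timeline lerps the root's scale from InitScale toward an offset built from the per-axis scale variables, with alpha divided by Size.
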(event `self.ReceiveBeginPlay`
  (add `self.OnSpawn` (delegate `SpawnAnimation`)))

(event `SpawnAnimation`
  (bind _defaultsceneroot (`self.DefaultSceneRoot`))
  (bind _initscale (`self.InitScale`))
  (bind _delay (`self.Delay`))
  (bind (_relativelocation_x _relativelocation_y _relativelocation_z) (`KismetMathLibrary.BreakVector` (`SceneComponent.RelativeLocation` (`self.DefaultSceneRoot`))))
  (`NiagaraFunctionLibrary.SpawnSystemAtLocation` "/Game/DepthScape/Virgile/VFX/NS_StingTrapV2.NS_StingTrapV2" (`KismetMathLibrary.MakeVector` _relativelocation_x _relativelocation_y (+ _relativelocation_z 10.0)))
  (`KismetSystemLibrary.Delay` 0.5)
  (bind (_direction _alpha) (`Timeline|Timeline`)
    (:`Update`
      (`SceneComponent.K2_SetRelativeTransform` _defaultsceneroot (`KismetMathLibrary.MakeTransform` (`SceneComponent.RelativeLocation` _defaultsceneroot) (`SceneComponent.RelativeRotation` _defaultsceneroot) (`KismetMathLibrary.VLerp` _initscale (+ _initscale (+ _delay (`self.xScale`)) (+ _delay (`self.yScale`)) (+ _delay (`self.zScale`))) (/ _alpha (`self.Size`)))) false false))))

(fn `UserConstructionScript`)