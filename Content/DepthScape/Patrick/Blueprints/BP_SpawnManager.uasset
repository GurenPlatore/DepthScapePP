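; BP_SpawnManager spawns BP_Watcher actors and tracks which watcher belongs to which spawn point.
; On BeginPlay it walks the keys of the SpawnPoints map, spawns a watcher at each key actor's transform and stores it as that key's value.
; RefreshSpawner takes a watcher reference, finds its spawn point by matching map values to keys, spawns a replacement there and overwrites the entry.
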(event `self.ReceiveBeginPlay`
  (`self.AwakeSpawn`))

(event `AwakeSpawn`
  (bind _keys (`BlueprintMapLibrary.Map_Keys` (`self.SpawnPoints`)))
  (for (_ _array_index) _keys
    (bind _keys_2 (`BlueprintMapLibrary.Map_Keys` (`self.SpawnPoints`)))
    (bind _output (`|GetArrayItem` _keys_2 _array_index))
    (bind _returnvalue (`|SpawnActorFromClass` "/Game/DepthScape/Patrick/Blueprints/Enemy/Watcher/BP_Watcher.BP_Watcher_C" (`self.GetTransform` _output) "Undefined" "MultiplyWithRoot" null null))
    (`BlueprintMapLibrary.Map_Add` (`self.SpawnPoints`) _output _returnvalue)))

(fn `RefreshSpawner`
  (params (WatcherRef :type "/Game/DepthScape/Patrick/Blueprints/Enemy/Watcher/BP_Watcher Object Reference"))
  (bind _values (`BlueprintMapLibrary.Map_Values` (`self.SpawnPoints`)))
  (bind _keys (`BlueprintMapLibrary.Map_Keys` (`self.SpawnPoints`)))
  (bind _output (`|GetArrayItem` _keys (`KismetArrayLibrary.Array_Find` _values WatcherRef)))
  (bind _returnvalue (`|SpawnActorFromClass` "/Game/DepthScape/Patrick/Blueprints/Enemy/Watcher/BP_Watcher.BP_Watcher_C" (`self.GetTransform` _output) "Undefined" "MultiplyWithRoot" null null))
  (`BlueprintMapLibrary.Map_Add` (`self.SpawnPoints`) _output _returnvalue))

(fn `UserConstructionScript`)