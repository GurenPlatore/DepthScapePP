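; BP_MutationsBath is a hub trigger actor for a mutations bath, with an unfinished enter/exit transition for the player.
; When BP_ProtoPatrick overlaps its Box, it stores the character, disables the box collision and calls SimpleMoveToLocation on the player controller.
; Mutation menu display and removal, collision restoring and movement disabling are unwired, as is the Destination location lookup.
; The exit branch only restores walking and is never called here.
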(event `self.Box.OnComponentBeginOverlap`
  (params (OverlappedComponent :type "PrimitiveComponent Object Reference") (OtherActor :type "Actor Object Reference") (OtherComp :type "PrimitiveComponent Object Reference") (OtherBodyIndex :type Integer) (bFromSweep :type Boolean) (SweepResult :type "HitResult Structure (by ref)"))
  (bind _asbp_proto_patrick (cast `/Game/DepthScape/Patrick/Blueprints/Character/BP_ProtoPatrick` OtherActor))
  (set `self.Proto Patrick` _asbp_proto_patrick)
  (`self.TransiInOutBath` true)
  (`self.AnimTransi`))

(event `self.Box.OnComponentEndOverlap`
  (params (OverlappedComponent :type "PrimitiveComponent Object Reference") (OtherActor :type "Actor Object Reference") (OtherComp :type "PrimitiveComponent Object Reference") (OtherBodyIndex :type Integer))
  (cast `/Game/DepthScape/Patrick/Blueprints/Character/BP_ProtoPatrick` OtherActor)
  (set `self.Proto Patrick` null))

(fn `AnimTransi`
  (`AIBlueprintHelperLibrary.SimpleMoveToLocation` (`GameplayStatics.GetPlayerController` 0) (`self.Goal`)))

(fn `TransiInOutBath`
  (params (In :type Boolean))
  (if In
    (`PrimitiveComponent.SetCollisionEnabled` (`self.Box`) "NoCollision")
    (else
      (`CharacterMovementComponent.SetMovementMode` (`Character.CharacterMovement` (`self.Proto Patrick`)) "MOVE_Walking" 0))))

(fn `UserConstructionScript`)