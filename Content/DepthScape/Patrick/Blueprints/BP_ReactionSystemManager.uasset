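; BP_ReactionSystemManager tracks the world's reaction to player actions as a five-tier level and shows its icon on the HUD.
; Detection, corpse detection, assimilation and environmental interaction each add their ratio to a gauge.
; A full gauge resets and raises the level, while an empty one lowers it.
; Level changes, plus a delayed BeginPlay call, refresh the icon through the player character's HUD widget.
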(event `self.ReceiveBeginPlay`
  (`KismetSystemLibrary.Delay` 1.0)
  (`self.UpdateTheNewReactionLevel`))

(fn `AddRemoveReactionPoints`
  (params (InfluenceType :type "/Game/DepthScape/Patrick/States/EReactionInfluences Enum" :default "NewEnumerator0"))
  (switch `/Game/DepthScape/Patrick/States/EReactionInfluences` InfluenceType
    (:`NewEnumerator0`
      (set `self.ReactionGauge` (+ (`self.DetectionRatio`) (`self.ReactionGauge`))))
    (:`NewEnumerator1`
      (set `self.ReactionGauge` (+ (`self.ReactionGauge`) (`self.CorpseDetectionRatio`))))
    (:`NewEnumerator2`
      (set `self.ReactionGauge` (+ (`self.ReactionGauge`) (`self.AssimiRatio`))))
    (:`NewEnumerator3`
      (set `self.ReactionGauge` (+ (`self.ReactionGauge`) (`self.EnviroInteractRatio`)))))
  (`self.CheckTheReactionLevel`))

(fn `CheckTheReactionLevel`
  (bind _reactionlevel (`self.ReactionLevel`))
  (bind _reactionlevel_2 (`self.ReactionLevel`))
  (if (>= (`self.ReactionGauge`) 1.0)
    (set `self.ReactionGauge` 0.0)
    (if (< _reactionlevel_2 4)
      (`/Engine/EditorBlueprintResources/StandardMacros.IncrementInt` _reactionlevel_2
        (:`  `
          (`self.UpdateTheNewReactionLevel` :!label _label))))
    (elif (<= (`self.ReactionGauge`) 0.0)
      (if (> _reactionlevel 0)
        (`/Engine/EditorBlueprintResources/StandardMacros.DecrementInt` _reactionlevel
          (:`  `
            (goto _label)))))))

(fn `GetReactionIcon`
  (returns (ReactionLevelIcon :type "Image Object Reference"))
  (return (`/Game/DepthScape/Patrick/Widgets/WBP_EmptyHUD.ReactionLevelIcon` (`/Game/DepthScape/Patrick/Widgets/WBP_CharacterHUD.WBP_EmptyHUD` (`/Game/DepthScape/Patrick/Blueprints/Character/BP_ProtoPatrick.CharacterHUDWidget` (cast `/Game/DepthScape/Patrick/Blueprints/Character/BP_ProtoPatrick` (`GameplayStatics.GetPlayerCharacter` 0) :!pure true))))))

(fn `UpdateTheNewReactionLevel`
  (switch `int` (`self.ReactionLevel`)
    (:`0`
      (bind _reactionlevelicon (`self.GetReactionIcon`))
      (`Image.SetBrushFromTexture` _reactionlevelicon (`|GetArrayItem` (`self.ReactionLevelIcons`) (`self.ReactionLevel`)) false))
    (:`1`
      (bind _reactionlevelicon_2 (`self.GetReactionIcon`))
      (`Image.SetBrushFromTexture` _reactionlevelicon_2 (`|GetArrayItem` (`self.ReactionLevelIcons`) (`self.ReactionLevel`)) false))
    (:`2`
      (bind _reactionlevelicon_3 (`self.GetReactionIcon`))
      (`Image.SetBrushFromTexture` _reactionlevelicon_3 (`|GetArrayItem` (`self.ReactionLevelIcons`) (`self.ReactionLevel`)) false))
    (:`3`
      (bind _reactionlevelicon_4 (`self.GetReactionIcon`))
      (`Image.SetBrushFromTexture` _reactionlevelicon_4 (`|GetArrayItem` (`self.ReactionLevelIcons`) (`self.ReactionLevel`)) false))
    (:`4`
      (bind _reactionlevelicon_5 (`self.GetReactionIcon`))
      (`Image.SetBrushFromTexture` _reactionlevelicon_5 (`|GetArrayItem` (`self.ReactionLevelIcons`) (`self.ReactionLevel`)) false))))

(fn `UserConstructionScript`)