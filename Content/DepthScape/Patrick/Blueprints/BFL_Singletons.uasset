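; Blueprint function library that gives global access to the level's manager actors: spawn, reaction system and mutations.
; Each getter checks whether its cached reference is valid and, if not, finds the actor with GetActorOfClass and stores it before returning it.
; The managers are only looked up, never spawned, so a getter returns null when no such actor exists in the world.
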(fn `GetMutationsManager`
  (returns (`Mutations Manager` :type "/Game/DepthScape/Patrick/Blueprints/Managers/BP_MutationsManager Object Reference"))
  (locals (MutationsManager :type "/Game/DepthScape/Patrick/Blueprints/Managers/BP_MutationsManager Object Reference"))
  (`/Engine/EditorBlueprintResources/StandardMacros.IsValid` (`local.MutationsManager`)
    (:`Is Valid`
      _)
    (:`Is Not Valid`
      (bind _returnvalue (`GameplayStatics.GetActorOfClass` null "/Game/DepthScape/Patrick/Blueprints/Managers/BP_MutationsManager.BP_MutationsManager_C"))
      (bind _output_get (set `local.MutationsManager` _returnvalue))))
  (return _output_get))

(fn `GetReactionSystemManager`
  (returns (`Reaction System Manager` :type "/Game/DepthScape/Patrick/Blueprints/Managers/BP_ReactionSystemManager Object Reference"))
  (locals (ReactionSystemManager :type "/Game/DepthScape/Patrick/Blueprints/Managers/BP_ReactionSystemManager Object Reference"))
  (`/Engine/EditorBlueprintResources/StandardMacros.IsValid` (`local.ReactionSystemManager`)
    (:`Is Valid`
      _)
    (:`Is Not Valid`
      (bind _returnvalue (`GameplayStatics.GetActorOfClass` null "/Game/DepthScape/Patrick/Blueprints/Managers/BP_ReactionSystemManager.BP_ReactionSystemManager_C"))
      (bind _output_get (set `local.ReactionSystemManager` _returnvalue))))
  (return _output_get))

(fn `GetSpawnManager`
  (returns (SpawnManagerRef :type "/Game/DepthScape/Patrick/Blueprints/Managers/BP_SpawnManager Object Reference"))
  (locals (SpawnManager :type "/Game/DepthScape/Patrick/Blueprints/Managers/BP_SpawnManager Object Reference"))
  (`/Engine/EditorBlueprintResources/StandardMacros.IsValid` (`local.SpawnManager`)
    (:`Is Valid`
      _)
    (:`Is Not Valid`
      (bind _returnvalue (`GameplayStatics.GetActorOfClass` null "/Game/DepthScape/Patrick/Blueprints/Managers/BP_SpawnManager.BP_SpawnManager_C"))
      (bind _output_get (set `local.SpawnManager` _returnvalue))))
  (return _output_get))