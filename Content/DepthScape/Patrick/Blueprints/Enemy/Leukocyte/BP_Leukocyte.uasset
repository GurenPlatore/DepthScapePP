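; Leukocyte enemy character that flies, is driven by an AI blackboard, and kills the player on overlap with its Box.
; BeginPlay sets the EnemyType key; Tick sets TargetActor to the player while detected and clears it otherwise.
; GetDown eases the mesh into a lowered, tilted pose once, guarded by SafetyLock.
; Chase and walk speed functions change MaxWalkSpeed, despite the Flying movement mode.
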(event `self.ReceiveBeginPlay`
  (`CharacterMovementComponent.SetMovementMode` (`self.CharacterMovement`) "MOVE_Flying" 0)
  (`BlackboardComponent.SetValueAsEnum` (`AIController.Blackboard` (`AIBlueprintHelperLibrary.GetAIController` self)) "EnemyType" (`self.EnemyType`))
  (bind _asbp_pyrite_character (cast `/Game/DepthScape/Patrick/Blueprints/Character/BP_PyriteCharacter` (`GameplayStatics.GetPlayerCharacter` 0)))
  (set `self.As BP Proto Patrick` _asbp_pyrite_character))

(event `self.ReceiveTick`
  (params (DeltaSeconds :type "Float (single-precision)"))
  (if (`/Game/DepthScape/Patrick/Blueprints/Character/BP_PyriteCharacter.IsDetected` (`self.As BP Proto Patrick`))
    (`BlackboardComponent.SetValueAsObject` (`AIController.Blackboard` (`AIBlueprintHelperLibrary.GetAIController` self)) "TargetActor" (`self.As BP Proto Patrick`))
    (else
      (`BlackboardComponent.SetValueAsObject` (`AIController.Blackboard` (`AIBlueprintHelperLibrary.GetAIController` self)) "TargetActor" null))))

(event `GetDown`
  (bind _mesh (`self.Mesh`))
  (bind (_relativelocation_x _relativelocation_y) (`KismetMathLibrary.BreakVector` (`SceneComponent.RelativeLocation` _mesh)))
  (if (not (`self.SafetyLock`))
    (set `self.SafetyLock` true)
    (`KismetSystemLibrary.MoveComponentTo` _mesh (`KismetMathLibrary.MakeVector` _relativelocation_x _relativelocation_y) (`KismetMathLibrary.MakeRotator` 40.0 0.0 -90.0) false true 3.0 true)))

(event `self.Box.OnComponentBeginOverlap`
  (params (OverlappedComponent :type "PrimitiveComponent Object Reference") (OtherActor :type "Actor Object Reference") (OtherComp :type "PrimitiveComponent Object Reference") (OtherBodyIndex :type Integer) (bFromSweep :type Boolean) (SweepResult :type "HitResult Structure (by ref)"))
  (bind _asbp_pyrite_character (cast `/Game/DepthScape/Patrick/Blueprints/Character/BP_PyriteCharacter` OtherActor))
  (`/Game/DepthScape/Patrick/Blueprints/Character/BP_PyriteCharacter.DeathEvent` _asbp_pyrite_character))

(event `self.Box.OnComponentEndOverlap`
  (params (OverlappedComponent :type "PrimitiveComponent Object Reference") (OtherActor :type "Actor Object Reference") (OtherComp :type "PrimitiveComponent Object Reference") (OtherBodyIndex :type Integer)))

(fn `SetChaseSpeed`
  (set `CharacterMovementComponent.MaxWalkSpeed` 900.0 (`self.CharacterMovement`)))

(fn `SetWalkSpeed`
  (set `CharacterMovementComponent.MaxWalkSpeed` 250.0 (`self.CharacterMovement`)))

(fn `UserConstructionScript`)