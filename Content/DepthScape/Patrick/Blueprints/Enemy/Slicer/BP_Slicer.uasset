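; BP_Slicer is a Slicer enemy actor that demolishes an array of wall actors.
; A Trigger overlap enables tick, whose timer destroys the first BreakWall entry each time BreakTime elapses.
; DeathEvent turns on mesh physics, disables custom depth and capsule collision, and changes State.
; Capsule overlaps only cast to BP_ProtoPatrick, and the widget and outline toggles are disconnected.
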(event `self.ReceiveTick`
  (params (DeltaSeconds :type "Float (single-precision)"))
  (bind _output (`|GetArrayItem` (`self.BreakWall`)))
  (bind _output_get (set `self.Timer` (+ (`self.Timer`) (`GameplayStatics.GetWorldDeltaSeconds`))))
  (if (> _output_get (`self.BreakTime`))
    (`/Engine/EditorBlueprintResources/StandardMacros.IsValid` _output
      (:`Is Valid`
        (`self.K2_DestroyActor` _output)
        (`KismetArrayLibrary.Array_Remove` (`self.BreakWall`))
        (set `self.Timer` 0.0)))))

(event `self.CapsuleComponent.OnComponentBeginOverlap`
  (params (OverlappedComponent :type "PrimitiveComponent Object Reference") (OtherActor :type "Actor Object Reference") (OtherComp :type "PrimitiveComponent Object Reference") (OtherBodyIndex :type Integer) (bFromSweep :type Boolean) (SweepResult :type "HitResult Structure (by ref)"))
  ;[1 1 1] Comment
  (cast `/Game/DepthScape/Patrick/Blueprints/Character/BP_ProtoPatrick` OtherActor))

(event `self.CapsuleComponent.OnComponentEndOverlap`
  (params (OverlappedComponent :type "PrimitiveComponent Object Reference") (OtherActor :type "Actor Object Reference") (OtherComp :type "PrimitiveComponent Object Reference") (OtherBodyIndex :type Integer))
  ;[1 1 1] Comment
  (cast `/Game/DepthScape/Patrick/Blueprints/Character/BP_ProtoPatrick` OtherActor))

(event `DeathEvent`
  (`PrimitiveComponent.SetSimulatePhysics` (`self.Mesh`) true)
  (`PrimitiveComponent.SetSimulatePhysics` (`self.tailleur_low`) true)
  (`PrimitiveComponent.SetRenderCustomDepth` (`self.Mesh`) false)
  (`PrimitiveComponent.SetRenderCustomDepth` (`self.tailleur_low`) false)
  (`PrimitiveComponent.SetCollisionEnabled` (`self.CapsuleComponent`) "NoCollision")
  (set `self.State` "NewEnumerator4"))

(event `self.trigger.OnActorBeginOverlap`
  (params (OverlappedActor :type "Actor Object Reference") (OtherActor :type "Actor Object Reference"))
  (`self.SetActorTickEnabled` true))

(fn `UserConstructionScript`)