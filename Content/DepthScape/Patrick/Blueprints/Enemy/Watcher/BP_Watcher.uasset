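; BP_Watcher is an AI enemy character that watches for the player with a traced line-of-sight mesh and can be killed.
; It writes spawn location, types and state to the Blackboard, switches patrol and chase speeds, and can sweep its yaw by Timeline.
; Detection percentage drives a progress widget.
; Overlaps toggle a custom-depth outline and grab-range state, while death enables physics, stops the vision mesh and disables collision.
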(event `VisibilityOn`
  (`SceneComponent.SetVisibility` (`self.Widget1`) true false))

(event `self.ReceiveBeginPlay`
  (bind _lineofsight (`self.LineOfSight`))
  ;[1 1 1] Comment
  (`|ExecutionSequence`
    (:`then_0`
      (`LineOfSightComponent.StartLineTrace` _lineofsight "TraceTypeQuery1" 40)
      (`LineOfSightComponent.StartBuildMesh` _lineofsight)
      (bind _returnvalue (`|CreateWidget` "/Game/DepthScape/Virgile/UI/Widgets/WBP_Detection.WBP_Detection_C"))
      (set `self.DetectionREF` _returnvalue)
      (`SceneComponent.SetVisibility` (`self.Widget1`) false false))
    (:`then_1`
      (`BlackboardComponent.SetValueAsVector` (`AIController.Blackboard` (`AIBlueprintHelperLibrary.GetAIController` self)) "SpawnLocation" (`self.K2_GetActorLocation`))
      (`KismetSystemLibrary.Delay` 1.0)
      (`BlackboardComponent.SetValueAsEnum` (`AIController.Blackboard` (`AIBlueprintHelperLibrary.GetAIController` self)) "WatcherType" (`self.WatcherType`))
      (`BlackboardComponent.SetValueAsEnum` (`AIController.Blackboard` (`AIBlueprintHelperLibrary.GetAIController` self)) "EnemyType" (`self.EnemyType`)))))

(event `PivotNCheck`
  ;[1 1 1] Comment
  (if (`|EnumEquality` (`self.WatcherType`) "NewEnumerator0")
    (bind (_direction _newtrack_1) (`Timeline|Timeline` :!label _label)
      (:`Update`
        (`self.K2_SetActorRotation` (`KismetMathLibrary.MakeRotator` 0.0 0.0 (`KismetMathLibrary.Lerp` 180.0 359.0 _newtrack_1)))))))

(event `StopTurn`
  ;[1 1 1] Comment
  (goto _label :!via `Stop`))

(event `DeathEvent`
  ;[1 1 1] Event when the Watcher get Killed
  (`self.SetDeadState`))

(event `self.CapsuleComponent.OnComponentBeginOverlap`
  (params (OverlappedComponent :type "PrimitiveComponent Object Reference") (OtherActor :type "Actor Object Reference") (OtherComp :type "PrimitiveComponent Object Reference") (OtherBodyIndex :type Integer) (bFromSweep :type Boolean) (SweepResult :type "HitResult Structure (by ref)"))
  ;[1 1 1] Comment
  (cast `/Game/DepthScape/Patrick/Blueprints/Character/BP_ProtoPatrick` OtherActor)
  (if (`|EnumInequality` (`self.WatcherState`) "NewEnumerator4")
    (`PrimitiveComponent.SetRenderCustomDepth` (`self.Mesh`) true)
    (`PrimitiveComponent.SetRenderCustomDepth` (`self.StaticMesh`) true)))

(event `self.CapsuleComponent.OnComponentEndOverlap`
  (params (OverlappedComponent :type "PrimitiveComponent Object Reference") (OtherActor :type "Actor Object Reference") (OtherComp :type "PrimitiveComponent Object Reference") (OtherBodyIndex :type Integer))
  ;[1 1 1] Comment
  (cast `/Game/DepthScape/Patrick/Blueprints/Character/BP_ProtoPatrick` OtherActor)
  (if (`|EnumInequality` (`self.WatcherState`) "NewEnumerator4")
    (`PrimitiveComponent.SetRenderCustomDepth` (`self.Mesh`) false)
    (`PrimitiveComponent.SetRenderCustomDepth` (`self.StaticMesh`) false)))

(event `self.GrabbingCollision.OnComponentBeginOverlap`
  (params (OverlappedComponent :type "PrimitiveComponent Object Reference") (OtherActor :type "Actor Object Reference") (OtherComp :type "PrimitiveComponent Object Reference") (OtherBodyIndex :type Integer) (bFromSweep :type Boolean) (SweepResult :type "HitResult Structure (by ref)"))
  (if (== OtherComp (`Character.CapsuleComponent` (cast `/Game/DepthScape/Patrick/Blueprints/Character/BP_ProtoPatrick` (`GameplayStatics.GetPlayerCharacter` 0) :!pure true)))
    (bind _asbp_proto_patrick (cast `/Game/DepthScape/Patrick/Blueprints/Character/BP_ProtoPatrick` OtherActor))
    (if (not (`/Game/DepthScape/Patrick/Blueprints/Character/BP_ProtoPatrick.EnemyInteract` _asbp_proto_patrick))
      (bind _output_get (set `self.WatcherState` "NewEnumerator6"))
      (`self.TransferStateToBT` _output_get "WatcherState")
      (`SceneComponent.SetVisibility` (`self.Widget`) false false)
      (`PrimitiveComponent.SetRenderCustomDepth` (`self.Mesh`) false))))

(event `Detecting`
  (params (PercentDetection :type "Float (double-precision)"))
  (bind _detectionref (`self.DetectionREF`))
  (bind _progressbar (`/Game/DepthScape/Virgile/UI/Widgets/WBP_Detection.ProgressBar` _detectionref))
  (bind _output_get (set `/Game/DepthScape/Virgile/UI/Widgets/WBP_Detection.Percentage Detection` PercentDetection _detectionref))
  (`ProgressBar.SetPercent` _progressbar _output_get)
  (`ProgressBar.SetFillColorAndOpacity` _progressbar (`/Game/DepthScape/Virgile/UI/Widgets/WBP_Detection.GetDetectionColor` _detectionref _output_get)))

(event `self.GrabbingCollision.OnComponentEndOverlap`
  (params (OverlappedComponent :type "PrimitiveComponent Object Reference") (OtherActor :type "Actor Object Reference") (OtherComp :type "PrimitiveComponent Object Reference") (OtherBodyIndex :type Integer))
  (cast `/Game/DepthScape/Patrick/Blueprints/Character/BP_ProtoPatrick` OtherActor))

(fn `EnableAssassination`
  (params (IsIne :type Boolean))
  (returns (isInTheBack :type Boolean))
  (if IsIne
    (bind _output_get (set `self.haveSomeoneBehind` true))
    (`self.StopTurn`)
    (return _output_get)
    (else
      (bind _output_get_2 (set `self.haveSomeoneBehind` false))
      (return _output_get_2))))

(fn `GrabbingPyriteEvent`
  (params (VisibilityMode :type Boolean))
  (returns (StaticMesh :type "StaticMeshComponent Object Reference"))
  (bind _staticmesh (`self.StaticMesh`))
  (`SceneComponent.SetVisibility` _staticmesh VisibilityMode false)
  (return _staticmesh))

(fn `SetChasingWalkSpeed`
  (set `CharacterMovementComponent.MaxWalkSpeed` (`self.ChasingWalkSpeed`) (`self.CharacterMovement`)))

(fn `SetDeadState`
  (bind _output_get (set `self.WatcherState` "NewEnumerator4"))
  (`self.TransferStateToBT` _output_get "WatcherState")
  (`PrimitiveComponent.SetSimulatePhysics` (`self.Mesh`) true)
  (`PrimitiveComponent.SetSimulatePhysics` (`self.StaticMesh`) true)
  (`LineOfSightComponent.StopBuildMesh` (`self.LineOfSight`))
  (`SceneComponent.SetVisibility` (`self.Widget`) false false)
  (`PrimitiveComponent.SetRenderCustomDepth` (`self.Mesh`) false)
  (`PrimitiveComponent.SetRenderCustomDepth` (`self.StaticMesh`) false)
  (`self.GrabbingPyriteEvent` true)
  (`PrimitiveComponent.SetCollisionEnabled` (`self.CapsuleComponent`) "NoCollision")
  (`PrimitiveComponent.SetCollisionEnabled` (`self.GrabbingCollision`) "NoCollision"))

(fn `SetPatrolWalkSpeed`
  (set `CharacterMovementComponent.MaxWalkSpeed` (`self.PatrolWalkSpeed`) (`self.CharacterMovement`)))

(fn `TransferStateToBT`
  (params (State :type "/Game/DepthScape/Patrick/States/EEnemyStates Enum" :default "NewEnumerator0") (Value :type Name))
  (`BlackboardComponent.SetValueAsEnum` (`AIController.Blackboard` (`AIBlueprintHelperLibrary.GetAIController` self)) (`KismetSystemLibrary.MakeLiteralName` Value) State))

(fn `UserConstructionScript`
  (`self.SetPatrolWalkSpeed`))