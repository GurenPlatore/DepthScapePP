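; Manager for the game's escalating reaction level, which responds to player-related events such as detection, corpse discovery and assimilation.
; Each event type adds its ratio to a gauge that steps the level between 0 and 4 at its limits.
; Level changes update the HUD icon, with camera shake above zero.
; Level 1 boosts watcher speed and detection, level 3 refreshes selected spawners, and level 4 shows the fail widget.
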(event `self.ReceiveBeginPlay`
  (bind _returnvalue (`|CreateWidget` "/Game/DepthScape/Virgile/UI/Widgets/WBP_FailWidget.WBP_FailWidget_C"))
  (set `self.FailWidgetREF` _returnvalue)
  (bind _returnvalue_2 (`|CreateWidget` "/Game/DepthScape/Virgile/UI/Widgets/Overlay/WBP_ShowFPS.WBP_ShowFPS_C"))
  (`UserWidget.AddToViewport` _returnvalue_2 0)
  (`KismetSystemLibrary.Delay` 0.5)
  (`self.UpdateTheNewReactionLevel`))

(fn `AddRemoveReactionPoints`
  (params (InfluenceType :type "/Game/DepthScape/Patrick/States/EReactionInfluences Enum" :default "NewEnumerator0"))
  (switch `/Game/DepthScape/Patrick/States/EReactionInfluences` InfluenceType
    (:`NewEnumerator0`
      (set `self.ReactionGauge` (+ (`self.DetectionRatio`) (`self.ReactionGauge`))))
    (:`NewEnumerator1`
      (set `self.ReactionGauge` (+ (`self.CorpseDetectionRatio`) (`self.ReactionGauge`))))
    (:`NewEnumerator2`
      (set `self.ReactionGauge` (+ (`self.AssimiRatio`) (`self.ReactionGauge`))))
    (:`NewEnumerator3`
      (set `self.ReactionGauge` (+ (`self.EnviroInteractRatio`) (`self.ReactionGauge`))))
    (:`NewEnumerator5`
      (set `self.ReactionGauge` (+ (`self.StickyRatio`) (`self.ReactionGauge`)))))
  (`self.CheckTheReactionLevel`))

(fn `ChangeSpeed &Detection`
  (bind _values (`BlueprintMapLibrary.Map_Values` (`/Game/DepthScape/Patrick/Blueprints/Managers/BP_SpawnManager.SpawnPoints` (`/Game/DepthScape/Patrick/Blueprints/BFL_Singletons.GetSpawnManager`))))
  (for _array_element _values
    (set `/Game/DepthScape/Patrick/Blueprints/Enemy/Watcher/BP_Watcher.ReactionWalkRatio` 1.4 _array_element)
    (`/Game/DepthScape/Patrick/Blueprints/Enemy/Watcher/BP_Watcher.SetPatrolWalkSpeed` _array_element)
    (set `/Game/DepthScape/Patrick/Blueprints/Enemy/Watcher/BP_Watcher.ReactionDetectionRatio` 1.5 _array_element)))

(fn `CheckTheReactionLevel`
  (bind _reactionlevel (`self.ReactionLevel`))
  (bind _reactionlevel_2 (`self.ReactionLevel`))
  (if (>= (`self.ReactionGauge`) 1.0)
    (set `self.ReactionGauge` 0.0)
    (if (< _reactionlevel_2 4)
      (`/Engine/EditorBlueprintResources/StandardMacros.IncrementInt` _reactionlevel_2
        (:`  `
          (`self.UpdateTheNewReactionLevel` :!label _label))))
    (elif (<= (`self.ReactionGauge`) 0.0)
      (if (> _reactionlevel 0)
        (`/Engine/EditorBlueprintResources/StandardMacros.DecrementInt` _reactionlevel
          (:`  `
            (goto _label)))))))

(fn `GetPyriteCharacter`
  (returns (`AsBP Pyrite Character` :type "/Game/DepthScape/Patrick/Blueprints/Character/BP_PyriteCharacter Object Reference"))
  (return (cast `/Game/DepthScape/Patrick/Blueprints/Character/BP_PyriteCharacter` (`GameplayStatics.GetPlayerCharacter` 0) :!pure true)))

(fn `GetReactionIcon`
  (returns (ReactionLevelIcon :type "Image Object Reference"))
  (return (`/Game/DepthScape/Patrick/Widgets/WBP_EmptyHUD.ReactionLevelIcon` (`/Game/DepthScape/Patrick/Widgets/WBP_CharacterHUD.WBP_EmptyHUD` (`/Game/DepthScape/Patrick/Blueprints/Character/BP_PyriteCharacter.CharacterHUDWidget` (cast `/Game/DepthScape/Patrick/Blueprints/Character/BP_PyriteCharacter` (`GameplayStatics.GetPlayerCharacter` 0) :!pure true))))))

(fn `UpdateTheNewReactionLevel`
  (bind _spawnmanagerref (`/Game/DepthScape/Patrick/Blueprints/BFL_Singletons.GetSpawnManager`))
  (bind _emptyhud (`self.EmptyHUD`))
  (switch `int` (`self.ReactionLevel`)
    (:`0`
      (bind _reactionlevelicon (`self.GetReactionIcon`))
      (`Image.SetBrushFromTexture` _reactionlevelicon (`|GetArrayItem` (`self.ReactionLevelIcons`) (`self.ReactionLevel`)) false))
    (:`1`
      (bind _reactionlevelicon_2 (`self.GetReactionIcon`))
      (`Image.SetBrushFromTexture` _reactionlevelicon_2 (`|GetArrayItem` (`self.ReactionLevelIcons`) (`self.ReactionLevel`)) false)
      (`/Game/DepthScape/Patrick/Blueprints/Character/BP_PyriteCharacter.StartCameraShake` (`self.GetPyriteCharacter`) "/Game/DepthScape/Virgile/Shake/CS_Reactions.CS_Reactions_C" "World")
      (`self.ChangeSpeed &Detection`)
      (`UserWidget.PlayAnimation` _emptyhud (`/Game/DepthScape/Patrick/Widgets/WBP_EmptyHUD.IncreaseReactionsLevels` _emptyhud) 0.0 1 "Forward" 1.0 false))
    (:`2`
      (bind _reactionlevelicon_3 (`self.GetReactionIcon`))
      (`Image.SetBrushFromTexture` _reactionlevelicon_3 (`|GetArrayItem` (`self.ReactionLevelIcons`) (`self.ReactionLevel`)) false)
      (`/Game/DepthScape/Patrick/Blueprints/Character/BP_PyriteCharacter.StartCameraShake` (`self.GetPyriteCharacter`) "/Game/DepthScape/Virgile/Shake/CS_Reactions.CS_Reactions_C" "World"))
    (:`3`
      (bind _reactionlevelicon_4 (`self.GetReactionIcon`))
      (`Image.SetBrushFromTexture` _reactionlevelicon_4 (`|GetArrayItem` (`self.ReactionLevelIcons`) (`self.ReactionLevel`)) false)
      (`/Game/DepthScape/Patrick/Blueprints/Character/BP_PyriteCharacter.StartCameraShake` (`self.GetPyriteCharacter`) "/Game/DepthScape/Virgile/Shake/CS_Reactions.CS_Reactions_C" "World")
      (bind _values (`BlueprintMapLibrary.Map_Values` (`/Game/DepthScape/Patrick/Blueprints/Managers/BP_SpawnManager.SpawnPoints` _spawnmanagerref)))
      (for _array_element _values
        (if (or (== _array_element null) (`|EnumEquality` (`/Game/DepthScape/Patrick/Blueprints/Enemy/Watcher/BP_Watcher.WatcherState` _array_element) "NewEnumerator4"))
          (`/Game/DepthScape/Patrick/Blueprints/Managers/BP_SpawnManager.RefreshSpawner` _spawnmanagerref _array_element))))
    (:`4`
      (bind _reactionlevelicon_5 (`self.GetReactionIcon`))
      (`Image.SetBrushFromTexture` _reactionlevelicon_5 (`|GetArrayItem` (`self.ReactionLevelIcons`) (`self.ReactionLevel`)) false)
      (`/Game/DepthScape/Patrick/Blueprints/Character/BP_PyriteCharacter.StartCameraShake` (`self.GetPyriteCharacter`) "/Game/DepthScape/Virgile/Shake/CS_Reactions.CS_Reactions_C" "World")
      (`UserWidget.AddToViewport` (`self.FailWidgetREF`) 0))))

(fn `UserConstructionScript`)