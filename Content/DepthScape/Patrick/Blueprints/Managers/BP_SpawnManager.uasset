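; Manager that spawns BP_Watcher enemies at mapped spawn points and can respawn, pause or unpause them.
; On BeginPlay it spawns a watcher per SpawnPoints key, copying that point's type, patrol and speed settings and storing the watcher as the map value.
; RefreshSpawner finds a given watcher's point by value lookup and spawns a replacement there.
; Pausing and unpausing toggle each watcher's CustomTimeDilation, with debug prints.
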(event `self.ReceiveTick`
  (params (DeltaSeconds :type "Float (single-precision)")))

(event `self.ReceiveBeginPlay`
  (`self.AwakeSpawn`))

(event `AwakeSpawn`
  (bind _keys (`BlueprintMapLibrary.Map_Keys` (`self.SpawnPoints`)))
  (for (_ _array_index) _keys
    (bind _keys_2 (`BlueprintMapLibrary.Map_Keys` (`self.SpawnPoints`)))
    (bind _output (`|GetArrayItem` _keys_2 _array_index))
    (bind (_returnvalue_location _returnvalue_rotation) (`KismetMathLibrary.BreakTransform` (`self.GetTransform` _output)))
    (bind _returnvalue (`|SpawnActorFromClass` "/Game/DepthScape/Patrick/Blueprints/Enemy/Watcher/BP_Watcher.BP_Watcher_C" (`KismetMathLibrary.MakeTransform` _returnvalue_location _returnvalue_rotation) "Undefined" "MultiplyWithRoot" null null))
    (set `/Game/DepthScape/Patrick/Blueprints/Enemy/Watcher/BP_SpawnPoint.WatcherSpawned` _returnvalue _output)
    (`BlueprintMapLibrary.Map_Add` (`self.SpawnPoints`) _output _returnvalue)
    (set `/Game/DepthScape/Patrick/Blueprints/Enemy/Watcher/BP_Watcher.WatcherType` (`/Game/DepthScape/Patrick/Blueprints/Enemy/Watcher/BP_SpawnPoint.WatcherType` _output) _returnvalue)
    (set `/Game/DepthScape/Patrick/Blueprints/Enemy/Watcher/BP_Watcher.PatrolPoints` (`/Game/DepthScape/Patrick/Blueprints/Enemy/Watcher/BP_SpawnPoint.PatrolPoints` _output) _returnvalue)
    (set `/Game/DepthScape/Patrick/Blueprints/Enemy/Watcher/BP_Watcher.PatrolMode` (`/Game/DepthScape/Patrick/Blueprints/Enemy/Watcher/BP_SpawnPoint.PatrolMode` _output) _returnvalue)
    (set `/Game/DepthScape/Patrick/Blueprints/Enemy/Watcher/BP_Watcher.PatrolWalkSpeed` (`/Game/DepthScape/Patrick/Blueprints/Enemy/Watcher/BP_SpawnPoint.PatrolWalkSpeed` _output) _returnvalue)
    (set `/Game/DepthScape/Patrick/Blueprints/Enemy/Watcher/BP_Watcher.ChasingWalkSpeed` (`/Game/DepthScape/Patrick/Blueprints/Enemy/Watcher/BP_SpawnPoint.ChasingWalkSpeed` _output) _returnvalue)))

(fn `PausedWatcher`
  (bind _values (`BlueprintMapLibrary.Map_Values` (`self.SpawnPoints`)))
  (for _array_element _values
    (bind _output_get (set `Actor.CustomTimeDilation` 0.0 _array_element))
    (`KismetSystemLibrary.PrintString` (`KismetStringLibrary.Conv_DoubleToString` _output_get))))

(fn `RefreshSpawner`
  (params (WatcherRef :type "/Game/DepthScape/Patrick/Blueprints/Enemy/Watcher/BP_Watcher Object Reference"))
  (bind _values (`BlueprintMapLibrary.Map_Values` (`self.SpawnPoints`)))
  (bind _keys (`BlueprintMapLibrary.Map_Keys` (`self.SpawnPoints`)))
  (bind _output (`|GetArrayItem` _keys (`KismetArrayLibrary.Array_Find` _values WatcherRef)))
  (bind _returnvalue (`|SpawnActorFromClass` "/Game/DepthScape/Patrick/Blueprints/Enemy/Watcher/BP_Watcher.BP_Watcher_C" (`self.GetTransform` _output) "Undefined" "MultiplyWithRoot" null null))
  (`BlueprintMapLibrary.Map_Add` (`self.SpawnPoints`) _output _returnvalue)
  (set `/Game/DepthScape/Patrick/Blueprints/Enemy/Watcher/BP_Watcher.WatcherType` (`/Game/DepthScape/Patrick/Blueprints/Enemy/Watcher/BP_SpawnPoint.WatcherType` _output) _returnvalue)
  (set `/Game/DepthScape/Patrick/Blueprints/Enemy/Watcher/BP_Watcher.PatrolPoints` (`/Game/DepthScape/Patrick/Blueprints/Enemy/Watcher/BP_SpawnPoint.PatrolPoints` _output) _returnvalue)
  (set `/Game/DepthScape/Patrick/Blueprints/Enemy/Watcher/BP_Watcher.PatrolMode` (`/Game/DepthScape/Patrick/Blueprints/Enemy/Watcher/BP_SpawnPoint.PatrolMode` _output) _returnvalue)
  (set `/Game/DepthScape/Patrick/Blueprints/Enemy/Watcher/BP_Watcher.PatrolWalkSpeed` (`/Game/DepthScape/Patrick/Blueprints/Enemy/Watcher/BP_SpawnPoint.PatrolWalkSpeed` _output) _returnvalue)
  (set `/Game/DepthScape/Patrick/Blueprints/Enemy/Watcher/BP_Watcher.ChasingWalkSpeed` (`/Game/DepthScape/Patrick/Blueprints/Enemy/Watcher/BP_SpawnPoint.ChasingWalkSpeed` _output) _returnvalue))

(fn `UnPausedWatcher`
  (bind _values (`BlueprintMapLibrary.Map_Values` (`self.SpawnPoints`)))
  (for _array_element _values
    (bind _output_get (set `Actor.CustomTimeDilation` 1.0 _array_element))
    (`KismetSystemLibrary.PrintString` (`KismetStringLibrary.Conv_DoubleToString` _output_get))))

(fn `UserConstructionScript`)