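; Mutations manager that runs the mutation bath enter/leave sequence and owns the mutations menu widget.
; EnterBath and LeaveBath drive the bath's collision and transition animation around timed delays, toggling the menu and cursor; leaving also restores game input and fades out the player's post-process.
; The construction script maps mutation enum values to skill components, and a helper reads rows from DT_Mutations.
; The UI-only input call is unwired, so entering never switches input mode.
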(event `self.ReceiveBeginPlay`
  (bind _returnvalue (`|CreateWidget` "/Game/DepthScape/Virgile/UI/Widgets/Menu/WBP_MutationsMenuV2.WBP_MutationsMenuV2_C"))
  (set `self.MutationMenuWidget` _returnvalue))

(event `EnterBath`
  (`/Game/DepthScape/Patrick/Blueprints/HUB/BP_MutationsBath.Open Close Bath Collision` (`self.MutationBath`) true)
  (`/Game/DepthScape/Patrick/Blueprints/HUB/BP_MutationsBath.AnimTransi` (`self.MutationBath`) true)
  (`KismetSystemLibrary.Delay` 2.5)
  (`self.Add Remove Widget` true))

(event `LeaveBath`
  (`self.Add Remove Widget` false)
  (`/Game/DepthScape/Patrick/Blueprints/HUB/BP_MutationsBath.AnimTransi` (`self.MutationBath`) false)
  (`KismetSystemLibrary.Delay` 2.5)
  (`/Game/DepthScape/Patrick/Blueprints/HUB/BP_MutationsBath.Open Close Bath Collision` (`self.MutationBath`) false)
  (`self.Set Input On UI Or Game` false)
  (`/Game/DepthScape/Patrick/Blueprints/Character/BP_PyriteCharacter.PostProcessWeightOutTransi` (cast `/Game/DepthScape/Patrick/Blueprints/Character/BP_PyriteCharacter` (`GameplayStatics.GetPlayerCharacter` 0) :!pure true)))

(fn `Add Remove Widget`
  (params (Condition :type Boolean))
  (bind _returnvalue (`GameplayStatics.GetPlayerController` 0))
  (if Condition
    (`UserWidget.AddToViewport` (`self.MutationMenuWidget`) 0)
    (set `PlayerController.bShowMouseCursor` true _returnvalue)
    (else
      (`Widget.RemoveFromParent` (`self.MutationMenuWidget`))
      (set `PlayerController.bShowMouseCursor` false _returnvalue))))

(fn `GetDataTableRowName`
  (params (NewParam :type Name))
  (returns (`Out Row` :type "/Game/DepthScape/Virgile/Data/SMutations Structure"))
  (bind _returnvalue (`|GetDataTableRow` "/Game/DepthScape/Virgile/Data/DT_Mutations.DT_Mutations" NewParam)
    (:`then`
      (return _returnvalue))))

(fn `MakeMapOfSkillComponents`
  (set `self.MutationComponentsByName` (`|MakeMap` "NewEnumerator9" (`self.AC_StingTrap`) "NewEnumerator8" (`self.AC_StunningSlingshot`) "NewEnumerator4" (`self.AC_CorpseDissolution`) "NewEnumerator11" (`self.AC_ChameleonCover`) "NewEnumerator12" (`self.AC_EnergeticStorage`) "NewEnumerator0" (`self.AC_AerialDive`) "NewEnumerator1" (`self.AC_Dash`) "NewEnumerator10" (`self.AC_MuffledSteps`) "NewEnumerator5" (`self.AC_AttractivePheromone`) "NewEnumerator13" (`self.AC_ChameleonClimb`) "NewEnumerator7" (`self.AC_Flash`) "NewEnumerator2" (`self.AC_RacingBlade`) "NewEnumerator3" (`self.AC_Slaughtering`) "NewEnumerator6" (`self.AC_Bloom`) :!type "/Game/DepthScape/Virgile/Data/EMutations Enum" :!valuetype "/Game/DepthScape/Patrick/Blueprints/AC_Mutations Object Reference")))

(fn `Set Input On UI Or Game`
  (params (Show :type Boolean))
  (bind _returnvalue (`GameplayStatics.GetPlayerController` 0))
  (if Show
    (`WidgetBlueprintLibrary.SetInputMode_UIOnlyEx` _returnvalue (`self.MutationMenuWidget`) "DoNotLock" true)
    (else
      (`WidgetBlueprintLibrary.SetInputMode_GameOnly` _returnvalue true))))

(fn `UserConstructionScript`
  (`self.MakeMapOfSkillComponents`))