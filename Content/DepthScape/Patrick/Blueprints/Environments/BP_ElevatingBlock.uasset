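; Interactable environment block that moves a referenced wall actor up, down, left or right as the player builds up interaction progress.
; A box overlap shows the interact widget; each Hold Interaction call adds progress and enables Tick, which drains it and lerps the wall from its start location.
; Near full progress it locks as complete, disables the box, fades the HUD outline, blends to a camera and back, and restores walking after a delay.
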(event `self.ReceiveTick`
  (params (DeltaSeconds :type "Float (single-precision)"))
  (if (`self.isComplete`)
    _
    (elif (== (`self.ProgressValue`) 0.0)
      (`self.SetActorTickEnabled` false)
      (`self.HideProgressBar`)
      (elif (`KismetMathLibrary.NearlyEqual_FloatFloat` (`self.ProgressValue`) 1.0 0.01)
        (`self.SetActorTickEnabled` false)
        (`PrimitiveComponent.SetCollisionEnabled` (`self.Box`) "NoCollision")
        (`SceneComponent.SetVisibility` (`self.WidgetInteraction`) false false)
        (`self.DisplayOutline`)
        (`PlayerController.SetViewTargetWithBlend` (`GameplayStatics.GetPlayerController` 0) (`self.Camera`) 3.0 "VTBlend_Cubic" 3.0 false)
        (`KismetSystemLibrary.Delay` (`self.Duration`))
        (`self.DisplayOutline`)
        (`PlayerController.SetViewTargetWithBlend` (`GameplayStatics.GetPlayerController` 0) (`GameplayStatics.GetPlayerCharacter` 0) 3.0 "VTBlend_Cubic" 3.0 false)
        (set `self.isComplete` true)
        (`KismetSystemLibrary.Delay` 3.0)
        (`CharacterMovementComponent.SetMovementMode` (`self.GetCharacterMovement`) "MOVE_Walking" 0)
        (else
          (`self.HoldInteraction` DeltaSeconds)
          (`self.Action Trigger`))))))

(event `self.ReceiveBeginPlay`
  (set `self.WallMeshLocation` (`self.K2_GetActorLocation` (`self.WallMesh`)))
  (`self.HideProgressBar`)
  (bind _returnvalue (`|CreateWidget` "/Game/DepthScape/Patrick/Widgets/WBP_CharacterHUD.WBP_CharacterHUD_C"))
  (set `self.CharacterHUD` _returnvalue))

(event `self.Box.OnComponentBeginOverlap`
  (params (OverlappedComponent :type "PrimitiveComponent Object Reference") (OtherActor :type "Actor Object Reference") (OtherComp :type "PrimitiveComponent Object Reference") (OtherBodyIndex :type Integer) (bFromSweep :type Boolean) (SweepResult :type "HitResult Structure (by ref)"))
  (cast `/Game/DepthScape/Patrick/Blueprints/Character/BP_PyriteCharacter` OtherActor)
  (`SceneComponent.SetVisibility` (`self.WidgetInteraction`) true false))

(event `self.Box.OnComponentEndOverlap`
  (params (OverlappedComponent :type "PrimitiveComponent Object Reference") (OtherActor :type "Actor Object Reference") (OtherComp :type "PrimitiveComponent Object Reference") (OtherBodyIndex :type Integer))
  (cast `/Game/DepthScape/Patrick/Blueprints/Character/BP_PyriteCharacter` OtherActor)
  (`SceneComponent.SetVisibility` (`self.WidgetInteraction`) false false))

(fn `Action Trigger`
  (switch `/Game/DepthScape/Virgile/Blueprints/EElevatingBlock` (`self.EElevatingBlock`)
    (:`NewEnumerator0`
      (`self.MoveUp`))
    (:`NewEnumerator1`
      (`self.MoveDown`))
    (:`NewEnumerator2`
      (`self.MoveRight`))
    (:`NewEnumerator3`
      (`self.MoveLeft`))))

(fn `DisplayOutline`
  (bind _characterhudwidget (`self.GetCharacterHUD`))
  (`WidgetSwitcher.SetActiveWidgetIndex` (`/Game/DepthScape/Patrick/Widgets/WBP_CharacterHUD.WidgetSwitcher_Outline` _characterhudwidget) 3)
  (`/Game/DepthScape/Virgile/UI/Widgets/WBP_Fade.FadeInFadeOut` (`/Game/DepthScape/Patrick/Widgets/WBP_CharacterHUD.WBP_Fade` _characterhudwidget)))

(fn `GetCharacterHUD`
  (returns (CharacterHUDWidget :type "/Game/DepthScape/Patrick/Widgets/WBP_CharacterHUD Object Reference"))
  (return (`/Game/DepthScape/Patrick/Blueprints/Character/BP_PyriteCharacter.CharacterHUDWidget` (cast `/Game/DepthScape/Patrick/Blueprints/Character/BP_PyriteCharacter` (`GameplayStatics.GetPlayerCharacter` 0) :!pure true))))

(fn `GetCharacterMovement`
  (returns (`Character Movement` :type "CharacterMovementComponent Object Reference"))
  (return (`Character.CharacterMovement` (cast `/Game/DepthScape/Patrick/Blueprints/Character/BP_PyriteCharacter` (`GameplayStatics.GetPlayerCharacter` 0) :!pure true))))

(fn `HideOutline`
  (`/Game/DepthScape/Virgile/UI/Widgets/WBP_Fade.FadeInFadeOut` (`/Game/DepthScape/Patrick/Widgets/WBP_CharacterHUD.WBP_Fade` (`self.GetCharacterHUD`))))

(fn `HideProgressBar`
  (`SceneComponent.SetVisibility` (`self.WidgetInteraction`) false false))

(fn `Hold Interaction`
  (`self.SetActorTickEnabled` true)
  (set `self.ProgressValue` (`KismetMathLibrary.FClamp` (+ (`self.ProgressValue`) 0.03))))

(fn `HoldInteraction`
  (params (Delta :type "Float (double-precision)"))
  (set `self.ProgressValue` (`KismetMathLibrary.FClamp` (- (`self.ProgressValue`) (/ Delta 3.0))))
  (bind _aswbp_interact (cast `/Game/DepthScape/Virgile/UI/Widgets/WBP_Interact` (`WidgetComponent.GetWidget` (`self.WidgetInteraction`))))
  (`/Game/DepthScape/Virgile/UI/Widgets/Overlay/WBP_CircularProgressBar.SetPercent` (`/Game/DepthScape/Virgile/UI/Widgets/WBP_Interact.WBP_ProgressBarMutation` _aswbp_interact) (`self.ProgressValue`)))

(fn `MoveCooldown`)

(fn `MoveDown`
  (bind (_wallmeshlocation_x _wallmeshlocation_y _wallmeshlocation_z) (`KismetMathLibrary.BreakVector` (`self.WallMeshLocation`)))
  (`self.K2_SetActorLocation` (`self.WallMesh`) (`KismetMathLibrary.MakeVector` _wallmeshlocation_x _wallmeshlocation_y (`KismetMathLibrary.Lerp` _wallmeshlocation_z (- _wallmeshlocation_z (`self.Z Pos to Move to`)) (`self.ProgressValue`))) false true))

(fn `MoveLeft`
  (bind (_wallmeshlocation_x _wallmeshlocation_y _wallmeshlocation_z) (`KismetMathLibrary.BreakVector` (`self.WallMeshLocation`)))
  (`self.K2_SetActorLocation` (`self.WallMesh`) (`KismetMathLibrary.MakeVector` (`KismetMathLibrary.Lerp` _wallmeshlocation_x (- _wallmeshlocation_x (`self.X Pos to Move to`)) (`self.ProgressValue`)) _wallmeshlocation_y _wallmeshlocation_z) false true))

(fn `MoveRight`
  (bind (_wallmeshlocation_x _wallmeshlocation_y _wallmeshlocation_z) (`KismetMathLibrary.BreakVector` (`self.WallMeshLocation`)))
  (`self.K2_SetActorLocation` (`self.WallMesh`) (`KismetMathLibrary.MakeVector` (`KismetMathLibrary.Lerp` _wallmeshlocation_x (+ _wallmeshlocation_x (`self.X Pos to Move to`)) (`self.ProgressValue`)) _wallmeshlocation_y _wallmeshlocation_z) false true))

(fn `MoveUp`
  (bind (_wallmeshlocation_x _wallmeshlocation_y _wallmeshlocation_z) (`KismetMathLibrary.BreakVector` (`self.WallMeshLocation`)))
  (`self.K2_SetActorLocation` (`self.WallMesh`) (`KismetMathLibrary.MakeVector` _wallmeshlocation_x _wallmeshlocation_y (`KismetMathLibrary.Lerp` _wallmeshlocation_z (+ _wallmeshlocation_z (`self.Z Pos to Move to`)) (`self.ProgressValue`))) false true))

(fn `UserConstructionScript`)