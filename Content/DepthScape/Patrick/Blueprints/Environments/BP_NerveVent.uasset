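; BP_NerveVent is an environment vent that can teleport the player to a linked destination.
; Its box overlap shows a widget while a BP_PyriteCharacter is inside and hides it on exit.
; TeleportThePlayer moves the passed character to DestinationRef's location and rotation as a teleport.
; PayToOpen only returns OpeningEnergyRatio; neither function is called within this Blueprint.
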(event `self.Box.OnComponentBeginOverlap`
  (params (OverlappedComponent :type "PrimitiveComponent Object Reference") (OtherActor :type "Actor Object Reference") (OtherComp :type "PrimitiveComponent Object Reference") (OtherBodyIndex :type Integer) (bFromSweep :type Boolean) (SweepResult :type "HitResult Structure (by ref)"))
  (cast `/Game/DepthScape/Patrick/Blueprints/Character/BP_PyriteCharacter` OtherActor)
  (`SceneComponent.SetVisibility` (`self.Widget`) true false))

(event `self.Box.OnComponentEndOverlap`
  (params (OverlappedComponent :type "PrimitiveComponent Object Reference") (OtherActor :type "Actor Object Reference") (OtherComp :type "PrimitiveComponent Object Reference") (OtherBodyIndex :type Integer))
  (cast `/Game/DepthScape/Patrick/Blueprints/Character/BP_PyriteCharacter` OtherActor)
  (`SceneComponent.SetVisibility` (`self.Widget`) false false))

(fn `PayToOpen`
  (returns (OpeningEnergyRatio :type "Float (double-precision)"))
  (return (`self.OpeningEnergyRatio`)))

(fn `TeleportThePlayer`
  (params (PlayerCharacter :type "/Game/DepthScape/Patrick/Blueprints/Character/BP_PyriteCharacter Object Reference"))
  (bind _destinationref (`self.DestinationRef`))
  (`self.K2_SetActorLocationAndRotation` PlayerCharacter (`self.K2_GetActorLocation` _destinationref) (`self.K2_GetActorRotation` _destinationref) false true))

(fn `UserConstructionScript`)