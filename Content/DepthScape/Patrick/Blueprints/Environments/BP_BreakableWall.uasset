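; BP_BreakableWall is a wall actor whose break action temporarily changes its surface rather than destroying it.
; DoTheBreakAction applies DiscMaterial to the static mesh, sets IsClean and enables actor tick.
; Tick accumulates DirtTimer for ten seconds, then restores the oak wood material, clears IsClean and disables tick.
; Repeated actions do not restart the running timer.
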(event `self.ReceiveTick`
  (params (DeltaSeconds :type "Float (single-precision)"))
  (bind _output_get (set `self.DirtTimer` (+ DeltaSeconds (`self.DirtTimer`))))
  (if (>= _output_get 10.0)
    (set `self.DirtTimer` 0.0)
    (`self.SetActorTickEnabled` false)
    (`PrimitiveComponent.SetMaterial` (`self.StaticMesh`) 0 "/Game/StarterContent/Materials/M_Wood_Oak.M_Wood_Oak")
    (set `self.IsClean` false)))

(fn `Do the Break Action`
  (`PrimitiveComponent.SetMaterial` (`self.StaticMesh`) 0 "/Engine/VREditor/UI/DiscMaterial.DiscMaterial")
  (set `self.IsClean` true)
  (`self.SetActorTickEnabled` true))

(fn `UserConstructionScript`)