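; BP_RessourcePlant is a resource plant whose bulb reappears a set time after being removed.
; RemoveBulbe&StartNewCycle hides the Bulbe component and enables actor tick, which is switched off at BeginPlay.
; Tick accumulates delta seconds until NewCycleTimer is reached, then shows the bulb, resets the count and disables itself, so the plant only ticks while regrowing.
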(event `self.ReceiveBeginPlay`
  (`self.SetActorTickEnabled` false))

(event `self.ReceiveTick`
  (params (DeltaSeconds :type "Float (single-precision)"))
  (bind _output_get (set `self.TimerCount` (+ (`self.TimerCount`) (`GameplayStatics.GetWorldDeltaSeconds`))))
  (if (>= _output_get (`self.NewCycleTimer`))
    (`self.SetActorTickEnabled` false)
    (`SceneComponent.SetVisibility` (`self.Bulbe`) true false)
    (set `self.TimerCount` 0.0)))

(event `Remove Bulbe & Start New Cycle`
  (`SceneComponent.SetVisibility` (`self.Bulbe`) false false)
  (`self.SetActorTickEnabled` true))

(fn `UserConstructionScript`
  (`parent.UserConstructionScript`))