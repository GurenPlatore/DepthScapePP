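; Alert bell that the player rings by holding an interaction, sending registered Watchers to investigate its location.
; Box overlap toggles the prompt widget, and each interaction call adds progress and enables Tick, which decays it and updates the progress bar.
; At completion it locks itself, restores player walking, and fills each Watcher's detection widget.
; It also writes a randomly offset bell location and new state to their AI Blackboards.
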(event `self.ReceiveBeginPlay`
  (set `self.ActualLocation` (`self.K2_GetActorLocation`)))

(event `self.Sphere.OnComponentBeginOverlap`
  (params (OverlappedComponent :type "PrimitiveComponent Object Reference") (OtherActor :type "Actor Object Reference") (OtherComp :type "PrimitiveComponent Object Reference") (OtherBodyIndex :type Integer) (bFromSweep :type Boolean) (SweepResult :type "HitResult Structure (by ref)"))
  (cast `/Game/DepthScape/Patrick/Blueprints/Character/BP_PyriteCharacter` OtherActor))

(event `Call Watchers`
  (bind (_actuallocation_x _actuallocation_y _actuallocation_z) (`KismetMathLibrary.BreakVector` (`self.ActualLocation`)))
  (for _array_element (`self.WatchersRef`)
    (`SceneComponent.SetVisibility` (`/Game/DepthScape/Patrick/Blueprints/Enemy/Watcher/BP_Watcher.DetectionWidget` _array_element) true false)
    (set `/Game/DepthScape/Virgile/UI/Widgets/WBP_Detection.Percentage Detection` 1.0 (cast `/Game/DepthScape/Virgile/UI/Widgets/WBP_Detection` (`WidgetComponent.GetWidget` (`/Game/DepthScape/Patrick/Blueprints/Enemy/Watcher/BP_Watcher.DetectionWidget` _array_element)) :!pure true))
    (bind _blackboard (`AIController.Blackboard` (`AIBlueprintHelperLibrary.GetAIController` _array_element)))
    (`BlackboardComponent.SetValueAsVector` _blackboard "LastKnownCharacterLocation" (`KismetMathLibrary.MakeVector` (+ _actuallocation_x (`KismetMathLibrary.RandomFloatInRange` -500.0 500.0)) (+ _actuallocation_y (`KismetMathLibrary.RandomFloatInRange` -500.0 500.0)) _actuallocation_z))
    (`BlackboardComponent.SetValueAsEnum` _blackboard "WatcherState" 2)))

(event `self.Box.OnComponentBeginOverlap`
  (params (OverlappedComponent :type "PrimitiveComponent Object Reference") (OtherActor :type "Actor Object Reference") (OtherComp :type "PrimitiveComponent Object Reference") (OtherBodyIndex :type Integer) (bFromSweep :type Boolean) (SweepResult :type "HitResult Structure (by ref)"))
  (cast `/Game/DepthScape/Patrick/Blueprints/Character/BP_PyriteCharacter` OtherActor)
  (`SceneComponent.SetVisibility` (`self.Widget`) true false))

(event `self.Box.OnComponentEndOverlap`
  (params (OverlappedComponent :type "PrimitiveComponent Object Reference") (OtherActor :type "Actor Object Reference") (OtherComp :type "PrimitiveComponent Object Reference") (OtherBodyIndex :type Integer))
  (cast `/Game/DepthScape/Patrick/Blueprints/Character/BP_PyriteCharacter` OtherActor)
  (`SceneComponent.SetVisibility` (`self.Widget`) false false))

(event `self.ReceiveTick`
  (params (DeltaSeconds :type "Float (single-precision)"))
  (if (`self.isComplete`)
    _
    (elif (== (`self.ProgressValue`) 0.0)
      (`self.SetActorTickEnabled` false)
      (elif (`KismetMathLibrary.NearlyEqual_FloatFloat` (`self.ProgressValue`) 1.0 0.01)
        (`self.SetActorTickEnabled` false)
        (`PrimitiveComponent.SetCollisionEnabled` (`self.Box`) "NoCollision")
        (`SceneComponent.SetVisibility` (`self.Widget`) false false)
        (set `self.isComplete` true)
        (`CharacterMovementComponent.SetMovementMode` (`self.GetCharacterMovement`) "MOVE_Walking" 0)
        (`self.Call Watchers`)
        (else
          (`self.Hold Interaction` DeltaSeconds))))))

(fn `AddToArray`
  (params (Watcher :type "/Game/DepthScape/Patrick/Blueprints/Enemy/Watcher/BP_Watcher Object Reference (by ref)"))
  (`KismetArrayLibrary.Array_Add` (`self.WatchersRef`) Watcher))

(fn `GetCharacterMovement`
  (returns (`Character Movement` :type "CharacterMovementComponent Object Reference"))
  (return (`Character.CharacterMovement` (cast `/Game/DepthScape/Patrick/Blueprints/Character/BP_PyriteCharacter` (`GameplayStatics.GetPlayerCharacter` 0) :!pure true))))

(fn `Hold Interaction`
  (params (Delta :type "Float (double-precision)"))
  (set `self.ProgressValue` (`KismetMathLibrary.FClamp` (- (`self.ProgressValue`) (/ Delta 3.0))))
  (bind _aswbp_interact (cast `/Game/DepthScape/Virgile/UI/Widgets/WBP_Interact` (`WidgetComponent.GetWidget` (`self.Widget`))))
  (`/Game/DepthScape/Virgile/UI/Widgets/Overlay/WBP_CircularProgressBar.SetPercent` (`/Game/DepthScape/Virgile/UI/Widgets/WBP_Interact.WBP_ProgressBarMutation` _aswbp_interact) (`self.ProgressValue`)))

(fn `HoldInteraction`
  (`self.SetActorTickEnabled` true)
  (set `self.ProgressValue` (`KismetMathLibrary.FClamp` (+ (`self.ProgressValue`) 0.03))))

(fn `UserConstructionScript`)