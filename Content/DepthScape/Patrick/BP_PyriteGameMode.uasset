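; Game mode for the Pyrite character that handles respawning through a destroyed-event handler.
; Respawn checks for the player's BP_PyriteCharacter and binds OnDestroy to an OnDestroyed event.
; OnDestroy switches the HUD outline widget, starts a fade-in, waits briefly, moves the player character to SpawnTransform without spawning a new one, then calls Respawn again.
; BeginPlay is empty, so nothing in this graph makes the first binding.
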(event `Respawn`
  (cast `/Game/DepthScape/Patrick/Blueprints/Character/BP_PyriteCharacter` (`GameplayStatics.GetPlayerCharacter` 0))
  (add `self.OnDestroyed` (delegate `OnDestroy`)))

(event `self.ReceiveBeginPlay`)

(event `OnDestroy` :!signature `self.OnDestroyed`
  (params (DestroyedActor :type "Actor Object Reference"))
  (bind _characterhudwidget (`/Game/DepthScape/Patrick/Blueprints/Character/BP_PyriteCharacter.CharacterHUDWidget` (cast `/Game/DepthScape/Patrick/Blueprints/Character/BP_PyriteCharacter` (`GameplayStatics.GetPlayerCharacter` 0) :!pure true)))
  (`WidgetSwitcher.SetActiveWidgetIndex` (`/Game/DepthScape/Patrick/Widgets/WBP_CharacterHUD.WidgetSwitcher_Outline` _characterhudwidget) 3)
  (`/Game/DepthScape/Virgile/UI/Widgets/WBP_Fade.Fade_In` (`/Game/DepthScape/Patrick/Widgets/WBP_CharacterHUD.WBP_Fade` _characterhudwidget))
  (`KismetSystemLibrary.Delay` 2.0)
  (`self.K2_SetActorTransform` (cast `/Game/DepthScape/Patrick/Blueprints/Character/BP_PyriteCharacter` (`GameplayStatics.GetPlayerCharacter` 0) :!pure true) (`self.SpawnTransform`) false false)
  (`self.Respawn`))

(fn `UserConstructionScript`)